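; Casement window Blueprint for a modular log house that opens automatically when a Character enters its trigger volume.
; A timeline drives the relative yaw of the left and right window meshes in opposite directions, swinging both open as a mirrored pair.
; The same timeline reverses when a Character leaves the trigger, closing the window.
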(event OnComponentBeginOverlap(Trigger_Window)
  (params (OverlappedComponent :type Primitive%20Component%20Object%20Reference) (OtherActor :type Actor%20Object%20Reference) (OtherComp :type Primitive%20Component%20Object%20Reference) (OtherBodyIndex :type Integer) (bFromSweep :type Boolean) (SweepResult :type Hit%20Result%20Structure%20%28by%20ref%29))
  (Utilities|Casting|CastToCharacter OtherActor)
  (bind _opendoor (Timeline|Timeline_1 Play)
    (:Update
      (Utilities|FlowControl|Sequence
        (:then_0
          (Transformation|SetRelativeRotation (Variables|Default|GetSM_Window_Left) (Math|Rotator|MakeRotator 0.0 0.0 (* _opendoor 1e+02)) false false))
        (:then_1
          (Transformation|SetRelativeRotation (Variables|Default|GetSM_Window_Right) (Math|Rotator|MakeRotator 0.0 0.0 (* (* _opendoor 1e+02) -1.0)) false false))))))

(event OnComponentEndOverlap(Trigger_Window)
  (params (OverlappedComponent :type Primitive%20Component%20Object%20Reference) (OtherActor :type Actor%20Object%20Reference) (OtherComp :type Primitive%20Component%20Object%20Reference) (OtherBodyIndex :type Integer))
  (Utilities|Casting|CastToCharacter OtherActor)
  (bind _opendoor (Timeline|Timeline_1 Reverse)
    (:Update
      (Utilities|FlowControl|Sequence
        (:then_0
          (Transformation|SetRelativeRotation (Variables|Default|GetSM_Window_Left) (Math|Rotator|MakeRotator 0.0 0.0 (* _opendoor 1e+02)) false false))
        (:then_1
          (Transformation|SetRelativeRotation (Variables|Default|GetSM_Window_Right) (Math|Rotator|MakeRotator 0.0 0.0 (* (* _opendoor 1e+02) -1.0)) false false))))))

(fn ConstructionScript)