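; Double door actor for modular log houses that swings open automatically when a Character enters its trigger volume.
; Trigger_Door overlap begin plays a timeline and overlap end reverses it to close the doors.
; The timeline's OpenDoor track drives the relative yaw of the left and right door meshes in opposite directions, scaled to a hard-coded maximum opening angle.
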(event OnComponentBeginOverlap(Trigger_Door)
  (params (OverlappedComponent :type Primitive%20Component%20Object%20Reference) (OtherActor :type Actor%20Object%20Reference) (OtherComp :type Primitive%20Component%20Object%20Reference) (OtherBodyIndex :type Integer) (bFromSweep :type Boolean) (SweepResult :type Hit%20Result%20Structure%20%28by%20ref%29))
  (Utilities|Casting|CastToCharacter OtherActor)
  (bind _opendoor (Timeline|Timeline_0 Play)
    (:Update
      (Utilities|FlowControl|Sequence
        (:then_0
          (Transformation|SetRelativeRotation (Variables|Default|GetSM_Door_L) (Math|Rotator|MakeRotator 0.0 0.0 (* _opendoor 1.5e+02)) false false))
        (:then_1
          (Transformation|SetRelativeRotation (Variables|Default|GetSM_Door_R) (Math|Rotator|MakeRotator 0.0 0.0 (* (* _opendoor 1.5e+02) -1.0)) false false))))))

(event OnComponentEndOverlap(Trigger_Door)
  (params (OverlappedComponent :type Primitive%20Component%20Object%20Reference) (OtherActor :type Actor%20Object%20Reference) (OtherComp :type Primitive%20Component%20Object%20Reference) (OtherBodyIndex :type Integer))
  (Utilities|Casting|CastToCharacter OtherActor)
  (bind _opendoor (Timeline|Timeline_0 Reverse)
    (:Update
      (Utilities|FlowControl|Sequence
        (:then_0
          (Transformation|SetRelativeRotation (Variables|Default|GetSM_Door_L) (Math|Rotator|MakeRotator 0.0 0.0 (* _opendoor 1.5e+02)) false false))
        (:then_1
          (Transformation|SetRelativeRotation (Variables|Default|GetSM_Door_R) (Math|Rotator|MakeRotator 0.0 0.0 (* (* _opendoor 1.5e+02) -1.0)) false false))))))

(fn ConstructionScript)